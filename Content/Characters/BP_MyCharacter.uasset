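; BP_MyCharacter is a character Blueprint with debug-key controls for spawning bullets and toggling a rifle between equipped and holstered.
; Debug key 2 spawns a BP_MyBullet at the spring arm's transform.
; Debug key H flip-flops IsEquipWeapon, playing the same equip montage both ways.
; After a fixed delay, the BP_MyBaseWeapon found through GetActorOfClass snaps to the mesh's Weapon or BackWeapon socket.
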(event EventBeginPlay)

(event Collision|EventActorBeginOverlap
  (params (OtherActor :type Actor%20Object%20Reference)))

(event EventTick
  (params (DeltaSeconds :type Float%20%28single-precision%29)))

(event Input|KeyboardEvents|DebugKey2
  (params (Key :type Key%20Structure :default "None") (ActionValue :type Input%20Action%20Value%20Structure))
  (:Pressed
    (Game|SpawnActorfromClass "/Game/Bullets/BP_MyBullet.BP_MyBullet_C" (Transformation|GetWorldTransform (Variables|Default|GetSpringArm)) "Undefined" "MultiplyWithRoot" 0 0)))

(event Input|KeyboardEvents|DebugKeyH
  (params (Key :type Key%20Structure :default "None") (ActionValue :type Input%20Action%20Value%20Structure))
  ;[1 1 1] EquipUnequipWeapon
  (:Pressed
    (Utilities|FlowControl|FlipFlop
      (:A
        (Variables|Default|SetbIsEquipWeapon true)
        (Animation|PlayAnimMontage "/Game/Characters/Animation/AM_Equip_Rifle_Standing.AM_Equip_Rifle_Standing" 1.0 "None")
        (Utilities|FlowControl|Delay 0.7)
        (bind _returnvalue (Actor|GetActorOfClass "/Game/Weapons/BP_MyBaseWeapon.BP_MyBaseWeapon_C"))
        (Transformation|AttachComponentToComponent _returnvalue (Variables|Character|GetMesh) "Weapon" "SnapToTarget" "SnapToTarget" "SnapToTarget" true))
      (:B
        (Variables|Default|SetbIsEquipWeapon false)
        (Animation|PlayAnimMontage "/Game/Characters/Animation/AM_Equip_Rifle_Standing.AM_Equip_Rifle_Standing" 1.0 "None")
        (Utilities|FlowControl|Delay 0.7)
        (bind _returnvalue_2 (Actor|GetActorOfClass "/Game/Weapons/BP_MyBaseWeapon.BP_MyBaseWeapon_C"))
        (Transformation|AttachComponentToComponent _returnvalue_2 (Variables|Character|GetMesh) "BackWeapon" "SnapToTarget" "SnapToTarget" "SnapToTarget" true)))))

(fn ConstructionScript)